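; OstrasizedGameMode is a game mode that respawns the player's OstrichCharacter whenever it is destroyed.
; On BeginPlay it binds to the OnDestroyed event of player 0's ostrich.
; When that fires, it spawns a new ostrich at SpawnTransform, turns off physics simulation on its capsule and has player controller 0 possess it.
; The Respawn event then loops back into the BeginPlay binding, so each new ostrich is watched in turn.
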(event `self.ReceiveBeginPlay`
  (bind _asostrich_character (cast `/Game/Ostrasized/Blueprints/OstrichCharacter` (`GameplayStatics.GetPlayerCharacter` 0) :!label _label))
  (add `self.OnDestroyed` _asostrich_character (delegate `OnDestroyed_0`)))

(event `OnDestroyed_0`
  (bind _returnvalue (`|SpawnActorFromClass` "/Game/Ostrasized/Blueprints/OstrichCharacter.OstrichCharacter_C" (`self.SpawnTransform`) "Undefined" "OverrideRootScale"))
  (`PrimitiveComponent.SetSimulatePhysics` (`Character.CapsuleComponent` _returnvalue) false)
  (`Controller.Possess` (`GameplayStatics.GetPlayerController` 0) _returnvalue)
  (`self.Respawn`))

(event `Respawn`
  (goto _label))

(fn `UserConstructionScript`)